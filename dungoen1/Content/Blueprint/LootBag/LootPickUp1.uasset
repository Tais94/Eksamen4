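; Loot pickup actor that rewards the player when a ThirdPersonMagicCharacter or PlayerCharacter overlaps it.
; On overlap it spawns the loot pickup particle at the overlapping character, then destroys itself.
; A small random amount is added to Currency for the magic character or Point for the PlayerCharacter.
; The reward always goes to player 0's character, cast to the matching class, rather than to the overlapping actor.
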(event EventBeginPlay)

(event Collision|EventActorBeginOverlap
  (params (OtherActor :type Actor%20Object%20Reference))
  (bind _asthird_person_magic_character (Utilities|Casting|CastToThirdPersonMagicCharacter OtherActor)
    (:then
      (Effects|SpawnEmitteratLocation "/Game/Blueprint/LootBag/P_Loot_Pickup.P_Loot_Pickup" (Transformation|GetActorLocation _asthird_person_magic_character))
      (bind _asthird_person_magic_character_2 (Utilities|Casting|CastToThirdPersonMagicCharacter (Game|GetPlayerCharacter 0)))
      (Variables|/Game/ThirdPersonBP/Blueprints/ThirdPersonMagicCharacter.ThirdPersonMagicCharacter_C|SetCurrency _asthird_person_magic_character_2 (+ (Variables|/Game/ThirdPersonBP/Blueprints/ThirdPersonMagicCharacter.ThirdPersonMagicCharacter_C|GetCurrency _asthird_person_magic_character_2) (Math|Random|RandomIntegerinRange 1 9)))
      (Actor|DestroyActor))
    (:CastFailed
      (bind _asplayer_character (Utilities|Casting|CastToPlayerCharacter OtherActor))
      (Effects|SpawnEmitteratLocation "/Game/Blueprint/LootBag/P_Loot_Pickup.P_Loot_Pickup" (Transformation|GetActorLocation _asplayer_character))
      (bind _asplayer_character_2 (Utilities|Casting|CastToPlayerCharacter (Game|GetPlayerCharacter 0)))
      (Variables|/Game/Player/PlayerCharacter.PlayerCharacter_C|SetPoint _asplayer_character_2 (+ (Variables|/Game/Player/PlayerCharacter.PlayerCharacter_C|GetPoint _asplayer_character_2) (Math|Random|RandomIntegerinRange 1 9)))
      (Actor|DestroyActor))))

(event EventTick
  (params (DeltaSeconds :type Float%20%28single-precision%29)))

(fn ConstructionScript)