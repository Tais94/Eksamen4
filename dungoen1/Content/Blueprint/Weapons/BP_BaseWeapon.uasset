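; Base melee weapon actor that loads its mesh and stats from a data table and line-traces for hits during attacks.
; StartAttack and EndAttack toggle per-tick multi-traces, using socket lookups (names currently None) if melee sockets exist, otherwise mesh bounds.
; Hits draw debug spheres and call GiveDamageOnce, whose check, as written, only damages actors already in HitActors.
; EndAttack clears that list.
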(event EventBeginPlay
  (bind _returnvalue (Utilities|GetDataTableRow "/Game/Blueprint/Weapons/WeaponTable.WeaponTable" (.RowName (Utilities|Struct|BreakDataTableRowHandle (Variables|Default|GetWeaponInDateTable))))
    (:then
      (bind _output_get (Variables|Default|SetWeaponInfo _returnvalue))
      (Class|SkinnedMeshComponent|SetSkeletalMesh (Variables|Default|GetWeaponMesh) (.WeaponMesh (Utilities|Struct|BreakFWeaponInfo _output_get)) true)
      (bind _havesockets (CallFunction|DoHaveSkeletonMesh))
      (Variables|Default|SetisUsingSockets _havesockets))))

(event Collision|EventActorBeginOverlap
  (params (OtherActor :type Actor%20Object%20Reference)))

(event EventTick
  (params (DeltaSeconds :type Float%20%28single-precision%29))
  (if (Variables|Default|GetIsInAttack)
    (bind (_outhits _returnvalue) (Class|KismetSystemLibrary|LineTraceMultiforObjects (stale _tracestart) (stale _trace_end) (Utilities|Array|MakeArray "ObjectTypeQuery1" "ObjectTypeQuery4" "ObjectTypeQuery2") true (Utilities|Array|MakeArray (Components|GetOwner)) "None" true))
    (if _returnvalue
      (bind _array_element (Utilities|Array|ForEachLoopwithBreak _outhits)
        (:LoopBody
          (Rendering|Debug|DrawDebugSphere (.ImpactPoint (Collision|BreakHitResult _array_element)) 1e+01 5 "(R=1.000000,G=1.000000,B=1.000000,A=1.000000)" 1.0 1.0)
          (CallFunction|GiveDamageOnce (.HitActor (Collision|BreakHitResult _array_element)) _array_element))))))

(fn ConstructionScript)

(fn StartAttack
  (Variables|Default|SetIsInAttack true))

(fn EndAttack
  (Variables|Default|SetIsInAttack false)
  (Utilities|Array|Clear (Variables|Default|GetHitActors)))

(fn DoHaveSkeletonMesh
  (return (and (Transformation|DoesSocketExist (Variables|Default|GetWeaponMesh) "MeleeStart") (Transformation|DoesSocketExist (Variables|Default|GetWeaponMesh) "MeleeEnd"))))

(fn GetTraceLocation
  (bind _weaponmesh (Variables|Default|GetWeaponMesh))
  (return (select (Variables|Default|GetisUsingSockets) (Transformation|GetSocketLocation (Variables|Default|GetWeaponMesh) "None") (Transformation|GetActorLocation)) (select (Variables|Default|GetisUsingSockets) (Transformation|GetSocketLocation (Variables|Default|GetWeaponMesh) "None") (+ (Transformation|GetActorLocation) (* (* (Math|Vector|GetUpVector _weaponmesh) -1.0) (* (.X (Math|Vector|BreakVector (.BoxExtent (Collision|GetComponentBounds _weaponmesh)))) (.DistanceModifier (Utilities|Struct|BreakFWeaponInfo (Variables|Default|GetWeaponInfo)))))))))

(fn GiveDamageOnce
  (params (To :type Actor%20Object%20Reference) (HitResult :type Hit%20Result%20Structure))
  (bind _hitactors (Variables|Default|GetHitActors))
  (if (Utilities|Array|IsValidIndex _hitactors (Utilities|Array|FindItem _hitactors To))
    (Utilities|Array|AddUnique (Variables|Default|GetHitActors) To)
    (Class|IDamage|TakeDamage(Message) To (.Damage (Utilities|Struct|BreakFWeaponInfo (Variables|Default|GetWeaponInfo))) HitResult (Components|GetOwner))))