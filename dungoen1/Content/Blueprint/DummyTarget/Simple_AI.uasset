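; Simple_AI is a dummy target character that takes damage from FireProjectile overlaps and rewards the player on death.
; Each overlap spawns a flame explosion, subtracts fixed Health and destroys the projectile.
; At zero Health, Death drops a LootPickUp at a toe socket, adds game mode Experience, handles level-ups with a doubling threshold and LevelUp widget, then destroys the actor.
; The TakeDamage spark function is never run.
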(event EventBeginPlay)

(event Collision|EventActorBeginOverlap
  (params (OtherActor :type Actor%20Object%20Reference))
  (bind _asfire_projectile (Utilities|Casting|CastToFireProjectile OtherActor))
  (Development|PrintString "HIT")
  (Effects|SpawnEmitteratLocation "/Game/InfinityBladeEffects/Effects/FX_Monsters/FX_Monster_Gruntling/FlameThrower/P_FlameExplode.P_FlameExplode" (Transformation|GetActorLocation _asfire_projectile))
  (bind _output_get (Variables|Default|SetHealth (- (Variables|Default|GetHealth) 0.25)))
  (if (<= _output_get 0.0)
    (CallFunction|Death)
    (Actor|DestroyActor _asfire_projectile)
    (else
      (Actor|DestroyActor _asfire_projectile))))

(event EventTick
  (params (DeltaSeconds :type Float%20%28single-precision%29)))

(fn ConstructionScript)

(fn TakeDamage
  (Effects|SpawnEmitteratLocation "/Game/InfinityBladeEffects/Effects/FX_Combat_Base/Impact/P_ImpactSpark.P_ImpactSpark" (Transformation|GetActorLocation)))

(fn Death
  (Game|SpawnActorfromClass "/Game/Blueprint/LootBag/LootPickUp.LootPickUp_C" (Math|Transform|MakeTransform (Transformation|GetSocketLocation (Variables|Character|GetMesh) "LeftToe_End")) "Undefined" 0 0)
  (bind _asthird_person_game_mode (Utilities|Casting|CastToThirdPersonGameMode (Game|GetGameMode)))
  (bind _output_get (Variables|/Game/ThirdPersonBP/Blueprints/ThirdPersonGameMode.ThirdPersonGameMode_C|SetExperience _asthird_person_game_mode (+ (Variables|/Game/ThirdPersonBP/Blueprints/ThirdPersonGameMode.ThirdPersonGameMode_C|GetExperience _asthird_person_game_mode) 1)))
  (if (>= _output_get (Variables|/Game/ThirdPersonBP/Blueprints/ThirdPersonGameMode.ThirdPersonGameMode_C|GetMaxExperiance _asthird_person_game_mode))
    (Variables|/Game/ThirdPersonBP/Blueprints/ThirdPersonGameMode.ThirdPersonGameMode_C|SetLevel _asthird_person_game_mode (+ (Variables|/Game/ThirdPersonBP/Blueprints/ThirdPersonGameMode.ThirdPersonGameMode_C|GetLevel _asthird_person_game_mode) 1))
    (Variables|/Game/ThirdPersonBP/Blueprints/ThirdPersonGameMode.ThirdPersonGameMode_C|SetExperience _asthird_person_game_mode 0)
    (Variables|/Game/ThirdPersonBP/Blueprints/ThirdPersonGameMode.ThirdPersonGameMode_C|SetMaxExperiance _asthird_person_game_mode (* (Variables|/Game/ThirdPersonBP/Blueprints/ThirdPersonGameMode.ThirdPersonGameMode_C|GetMaxExperiance _asthird_person_game_mode) 2))
    (bind _returnvalue (Game|ConstructObjectfromClass "/Game/ThirdPersonBP/Blueprints/LevelUp.LevelUp_C" (Game|GetPlayerCharacter 0)))
    (UserInterface|Viewport|AddtoViewport _returnvalue 0))
  (bind _asthird_person_game_mode_2 (Utilities|Casting|CastToThirdPersonGameMode (Game|GetGameMode)))
  (Default|UpdateNumbers _asthird_person_game_mode_2)
  (Actor|DestroyActor))