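; Health pickup actor that heals the player character on overlap.
; On overlap with a ThirdPersonMagicCharacter whose Health is not above full, it adds a fixed amount and clamps the result to the maximum.
; It then spawns a heal potion particle effect at the character's location and destroys itself.
; A character at exactly full health still consumes the pickup, as only values above the maximum are rejected.
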(event EventBeginPlay)

(event Collision|EventActorBeginOverlap
  (params (OtherActor :type Actor%20Object%20Reference))
  (bind _asthird_person_magic_character (Utilities|Casting|CastToThirdPersonMagicCharacter OtherActor))
  (if (not (> (Variables|/Game/ThirdPersonBP/Blueprints/ThirdPersonMagicCharacter.ThirdPersonMagicCharacter_C|GetHealth _asthird_person_magic_character) 1.0))
    (bind _output_get (Variables|/Game/ThirdPersonBP/Blueprints/ThirdPersonMagicCharacter.ThirdPersonMagicCharacter_C|SetHealth _asthird_person_magic_character (+ (Variables|/Game/ThirdPersonBP/Blueprints/ThirdPersonMagicCharacter.ThirdPersonMagicCharacter_C|GetHealth _asthird_person_magic_character) 0.2)))
    (if (> _output_get 1.0)
      (Variables|/Game/ThirdPersonBP/Blueprints/ThirdPersonMagicCharacter.ThirdPersonMagicCharacter_C|SetHealth _asthird_person_magic_character 1.0))
    (Effects|SpawnEmitteratLocation "/Game/Blueprint/HealthPickUp/P_Heal_Potion.P_Heal_Potion" (Transformation|GetActorLocation _asthird_person_magic_character))
    (Actor|DestroyActor)))

(event EventTick
  (params (DeltaSeconds :type Float%20%28single-precision%29)))

(fn ConstructionScript)