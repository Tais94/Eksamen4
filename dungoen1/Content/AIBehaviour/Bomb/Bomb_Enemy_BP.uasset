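; Bomb enemy character that chases a seen, living player and self-destructs at close range or when a Weapon overlaps its capsule.
; Pawn sensing drives an AI MoveTo, with a retriggerable delay clearing InRange after the move succeeds or fails.
; Both detonation paths stop movement, set Attack, wait, then fire a radial impulse and particles before destroying the actor.
; Health damage applies only if the player is within range when checked, before the final fuse delay.
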(event OnSeePawn(PawnSensing)
  (params (Pawn :type Pawn%20Object%20Reference))
  ;[1 1 1] Follow player
  (bind _asplayer_character (Utilities|Casting|CastToPlayerCharacter Pawn))
  (if (not (Variables|/Game/Player/PlayerCharacter.PlayerCharacter_C|GetIsDead _asplayer_character))
    (Variables|Default|SetinRange true)
    (AI|AIMoveTo self "0, 0, 0" _asplayer_character 1e+02 false
      (:then
        (Variables|Default|SetinRange true)
        ;[1 1 1] Get distance and wait, attack
        (bind _output_get (Variables|Default|SetAttackRange (Transformation|GetDistanceTo (Game|Player|GetPlayerPawn 0))))
        (if (<= _output_get 1.5e+02)
          (Pawn|Components|CharacterMovement|DisableMovement (Variables|Character|GetCharacterMovement))
          (AI|Navigation|StopMovement (Pawn|GetController))
          (Utilities|FlowControl|Delay 1.0)
          (Variables|Default|SetAttack true)
          ;[1 1 1] damage Player
          (if (<= (Transformation|GetDistanceTo (Game|Player|GetPlayerPawn 0)) 1.5e+02)
            (Utilities|FlowControl|Delay 1.2)
            (Utilities|FlowControl|DoOnce false
              (:Completed
                (bind _asplayer_character_2 (Utilities|Casting|CastToPlayerCharacter (Game|GetPlayerCharacter 0)))
                (Variables|/Game/Player/PlayerCharacter.PlayerCharacter_C|SetHealth _asplayer_character_2 (- (Variables|/Game/Player/PlayerCharacter.PlayerCharacter_C|GetHealth _asplayer_character_2) 5e+01))))
            (else
              (Utilities|FlowControl|Delay 1.2)))
          ;[1 1 1] Comment
          (Utilities|FlowControl|Sequence
            (:then_0
              (Class|RadialForceComponent|FireImpulse (Variables|Default|GetRadialForce))
              (Utilities|FlowControl|Delay 0.5)
              (Actor|DestroyActor))
            (:then_1
              (Components|Activation|Activate (Variables|Default|GetParticleSystem) false)))))
      (:OnSuccess
        (Utilities|FlowControl|RetriggerableDelay 4.0 :!label _label)
        (Variables|Default|SetinRange false))
      (:OnFail
        (goto _label)))))

(event OnComponentBeginOverlap(CapsuleComponent)
  (params (OverlappedComponent :type Primitive%20Component%20Object%20Reference) (OtherActor :type Actor%20Object%20Reference) (OtherComp :type Primitive%20Component%20Object%20Reference) (OtherBodyIndex :type Integer) (bFromSweep :type Boolean) (SweepResult :type Hit%20Result%20Structure%20%28by%20ref%29))
  (Utilities|Casting|CastToWeapon OtherActor)
  (Pawn|Components|CharacterMovement|DisableMovement (Variables|Character|GetCharacterMovement))
  (AI|Navigation|StopMovement (Pawn|GetController))
  (Variables|Default|SetAttack true)
  ;[1 1 1] damage Player
  (if (<= (Transformation|GetDistanceTo (Game|Player|GetPlayerPawn 0)) 1.5e+02)
    (Utilities|FlowControl|Delay 1.2)
    (Utilities|FlowControl|DoOnce false
      (:Completed
        (bind _asplayer_character (Utilities|Casting|CastToPlayerCharacter (Game|GetPlayerCharacter 0)))
        (Variables|/Game/Player/PlayerCharacter.PlayerCharacter_C|SetHealth _asplayer_character (- (Variables|/Game/Player/PlayerCharacter.PlayerCharacter_C|GetHealth _asplayer_character) 5e+01))))
    (else
      (Utilities|FlowControl|Delay 1.2)))
  (Utilities|FlowControl|Sequence
    (:then_0
      (Class|RadialForceComponent|FireImpulse (Variables|Default|GetRadialForce))
      (Utilities|FlowControl|Delay 0.5)
      (Actor|DestroyActor))
    (:then_1
      (Components|Activation|Activate (Variables|Default|GetParticleSystem) false))))

(event EventBeginPlay)

(event Collision|EventActorBeginOverlap
  (params (OtherActor :type Actor%20Object%20Reference)))

(event EventTick
  (params (DeltaSeconds :type Float%20%28single-precision%29)))

(fn ConstructionScript)