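; Minion enemy pawn that wanders navmesh points, chases the melee or magic player on sight and attacks up close.
; Overlaps handle weapon hits both ways and fireball damage.
; Tick drives wandering, death, the camera-facing health bar and player references, polling the melee player's attack state.
; Death drops loot and awards game-mode XP with level-ups, but only when the melee reference is valid, as both branches check it.
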(event OnSeePawn(PawnSensing)
  (params (Pawn :type Pawn%20Object%20Reference))
  (bind _meleeref (Variables|Default|GetMeleeRef))
  (bind _magicref (Variables|Default|GetMagicRef))
  (Utilities|FlowControl|Sequence
    (:then_0
      ;[1 1 1] Follow Player on see
      (Utilities|IsValid _meleeref
        (:Is%20Valid
          (if (not (Variables|/Game/Player/PlayerCharacter.PlayerCharacter_C|GetIsDead _meleeref))
            (Variables|Default|SetinRange true)
            (AI|AIMoveTo self "0, 0, 0" _meleeref 1.4e+02 false
              (:then
                (Variables|Default|SetinRange true)
                ;[1 1 1] Attack Player
                (Variables|Default|SetAttackRange (Transformation|GetDistanceTo (Game|Player|GetPlayerPawn 0)) :!label _label)
                (if (<= (Variables|Default|GetAttackRange) 1.5e+02)
                  (Variables|Default|SetCanAttack true)
                  (Pawn|Components|CharacterMovement|DisableMovement (Variables|Character|GetCharacterMovement))
                  (Utilities|FlowControl|Delay 0.48)
                  (Variables|Default|SetCanAttack false)
                  (Pawn|Components|CharacterMovement|SetMovementMode (Variables|Character|GetCharacterMovement) "MOVE_Walking" 0)))
              (:OnSuccess
                (Utilities|FlowControl|RetriggerableDelay 4.0 :!label _label_2)
                (Variables|Default|SetinRange false))
              (:OnFail
                (goto _label_2)))))
        (:Is%20Not%20Valid
          ;[1 1 1] Follow magicplayer on see
          (Utilities|IsValid _magicref
            (:Is%20Valid
              (if (not (Variables|/Game/ThirdPersonBP/Blueprints/ThirdPersonMagicCharacter.ThirdPersonMagicCharacter_C|GetIsDead _magicref))
                (Variables|Default|SetinRange true)
                (AI|AIMoveTo self "0, 0, 0" _magicref 1.4e+02 false
                  (:then
                    (Variables|Default|SetinRange true)
                    (goto _label))
                  (:OnSuccess
                    _)
                  (:OnFail
                    _))
                (Utilities|FlowControl|RetriggerableDelay 4.0)
                (Variables|Default|SetinRange false)))))))
    (:then_1
      ;[1 1 1] stop following player if dead
      (if (Variables|Default|GetIsDead)
        (Components|Movement|StopMovementImmediately (Variables|Character|GetCharacterMovement))))))

(event OnComponentBeginOverlap(WeaponCollision)
  (params (OverlappedComponent :type Primitive%20Component%20Object%20Reference) (OtherActor :type Actor%20Object%20Reference) (OtherComp :type Primitive%20Component%20Object%20Reference) (OtherBodyIndex :type Integer) (bFromSweep :type Boolean) (SweepResult :type Hit%20Result%20Structure%20%28by%20ref%29))
  ;[1 1 1] Weapon Collision
  (Utilities|IsValid (Variables|Default|GetMeleeRef)
    (:Is%20Valid
      (bind _asplayer_character (Utilities|Casting|CastToPlayerCharacter OtherActor))
      (if (Variables|Default|GetCanAttack)
        (if (Variables|Default|GetHitOnce)
          (Variables|/Game/Player/PlayerCharacter.PlayerCharacter_C|SetHealth _asplayer_character (- (Variables|/Game/Player/PlayerCharacter.PlayerCharacter_C|GetHealth _asplayer_character) 5.0))
          (Variables|Default|SetHitOnce false)
          (else
            (Utilities|FlowControl|Delay 0.25)
            (Variables|Default|SetHitOnce true)))))
    (:Is%20Not%20Valid
      (Utilities|IsValid (Variables|Default|GetMagicRef)
        (:Is%20Valid
          (bind _asthird_person_magic_character (Utilities|Casting|CastToThirdPersonMagicCharacter OtherActor))
          (if (Variables|Default|GetCanAttack)
            (if (Variables|Default|GetHitOnce)
              (Variables|/Game/ThirdPersonBP/Blueprints/ThirdPersonMagicCharacter.ThirdPersonMagicCharacter_C|SetHealth _asthird_person_magic_character (- (Variables|/Game/ThirdPersonBP/Blueprints/ThirdPersonMagicCharacter.ThirdPersonMagicCharacter_C|GetHealth _asthird_person_magic_character) 5.0))
              (Variables|Default|SetHitOnce false)
              (else
                (Utilities|FlowControl|Delay 0.25)
                (Variables|Default|SetHitOnce true)))))))))

(event OnComponentBeginOverlap(CapsuleComponent)
  (params (OverlappedComponent :type Primitive%20Component%20Object%20Reference) (OtherActor :type Actor%20Object%20Reference) (OtherComp :type Primitive%20Component%20Object%20Reference) (OtherBodyIndex :type Integer) (bFromSweep :type Boolean) (SweepResult :type Hit%20Result%20Structure%20%28by%20ref%29))
  ;[1 1 1] take damage
  (Utilities|Casting|CastToWeapon OtherActor)
  (if (Variables|Default|GetEnemyAttacking)
    (if (Variables|Default|GetHitOnce)
      (Utilities|FlowControl|Delay 1.0)
      (Variables|Default|SetHitOnce false)
      (else
        (Variables|Default|SetHitOnce true)
        (Utilities|FlowControl|Delay 0.4)
        (Variables|Default|SetHealth (- (Variables|Default|GetHealth) 5e+01))))))

(event EventTick
  (params (DeltaSeconds :type Float%20%28single-precision%29))
  (bind _rotation_ancor (Variables|Default|GetRotation%20ancor))
  (Utilities|FlowControl|Sequence
    (:then_0
      ;[1 1 1] Get Random location
      (if (not (Variables|Default|GetinRange))
        (if (not (Variables|Default|GetMoving))
          (AI|AIMoveTo self (.RandomLocation (Class|NavigationSystem|GetRandomPointinNavigableRadius (Transformation|GetActorLocation) 4e+02)) 0 5.0 false
            (:then
              (Variables|Default|SetMoving true))
            (:OnSuccess
              (Variables|Default|SetMoving false :!label _label))
            (:OnFail
              (goto _label))))))
    (:then_1
      ;[1 1 1] Death
      (if (<= (Variables|Default|GetHealth) 0.0)
        (Variables|Default|SetIsDead true)
        (Components|Movement|StopMovementImmediately (Variables|Character|GetCharacterMovement))
        (Utilities|FlowControl|DoOnce false
          (:Completed
            ;[1 1 1] point
            (Utilities|IsValid (Variables|Default|GetMeleeRef)
              (:Is%20Valid
                _)
              (:Is%20Not%20Valid
                (Utilities|IsValid (Variables|Default|GetMeleeRef)
                  (:Is%20Valid
                    _))))
            (Utilities|FlowControl|Delay 2.067)
            (CallFunction|DeathLootXP)
            (Actor|DestroyActor)))))
    (:then_2
      ;[1 1 1] rotate widget
      (Transformation|SetWorldRotation _rotation_ancor (Math|Rotator|MakeRotator 0.0 0.0 (.Yaw (Math|Rotator|BreakRotator (Math|Rotator|FindLookatRotation (Transformation|GetWorldLocation _rotation_ancor) (Transformation|GetActorLocation (Game|GetPlayerCameraManager 0)))))) false false))
    (:then_3
      ;[1 1 1] Health widget
      (bind _asenemy_health (Utilities|Casting|CastToEnemyHealth (UserInterface|GetUserWidgetObject (Variables|Default|GetHealthBar))))
      (bind _output_get (Variables|Default|SetUIHealth _asenemy_health))
      (Progress|SetPercent (Variables|/Game/UI/EnemyHealth.EnemyHealth_C|GetProgressBar_73 _output_get) (/ (Variables|Default|GetHealth) 1e+02)))
    (:then_4
      ;[1 1 1] Player Attack bool
      (bind _asplayer_character (Utilities|Casting|CastToPlayerCharacter (Game|GetPlayerCharacter 0)))
      (Variables|Default|SetEnemyAttacking (Variables|/Game/Player/PlayerCharacter.PlayerCharacter_C|GetAttacking _asplayer_character)))
    (:then_5
      ;[1 1 1] Create player refs
      (bind _outactors (Actor|GetAllActorswithTag "Player"))
      (for (_array_element _array_index) _outactors
        (if (Actor|ActorHasTag _array_element (Utilities|Array|Get(acopy) (Variables|/Script/Engine.Actor|GetTags _array_element) _array_index))
          (bind _asthird_person_magic_character (Utilities|Casting|CastToThirdPersonMagicCharacter _array_element)
            (:then
              (Variables|Default|SetMagicRef _asthird_person_magic_character))
            (:CastFailed
              (bind _asplayer_character_2 (Utilities|Casting|CastToPlayerCharacter (Game|GetPlayerCharacter 0)))
              (Variables|Default|SetMeleeRef _asplayer_character_2))))))))

(event Collision|EventActorBeginOverlap
  (params (OtherActor :type Actor%20Object%20Reference))
  ;[1 1 1] Take Magic Damage
  (bind _asfire_projectile (Utilities|Casting|CastToFireProjectile OtherActor))
  (Effects|SpawnEmitteratLocation "/Game/InfinityBladeEffects/Effects/FX_Monsters/FX_Monster_Gruntling/FlameThrower/P_FlameExplode.P_FlameExplode" (Transformation|GetActorLocation _asfire_projectile))
  (Variables|Default|SetHealth (- (Variables|Default|GetHealth) 35.0)))

(fn ConstructionScript)

(fn DeathLootXP
  (Game|SpawnActorfromClass "/Game/Blueprint/LootBag/LootPickUp.LootPickUp_C" (Math|Transform|MakeTransform (Transformation|GetSocketLocation (Variables|Character|GetMesh) "head")) "Undefined" 0 0)
  (bind _asthird_person_game_mode (Utilities|Casting|CastToThirdPersonGameMode (Game|GetGameMode)))
  (bind _output_get (Variables|/Game/ThirdPersonBP/Blueprints/ThirdPersonGameMode.ThirdPersonGameMode_C|SetExperience _asthird_person_game_mode (+ (Variables|/Game/ThirdPersonBP/Blueprints/ThirdPersonGameMode.ThirdPersonGameMode_C|GetExperience _asthird_person_game_mode) 1)))
  (if (>= _output_get (Variables|/Game/ThirdPersonBP/Blueprints/ThirdPersonGameMode.ThirdPersonGameMode_C|GetMaxExperiance _asthird_person_game_mode))
    (Variables|/Game/ThirdPersonBP/Blueprints/ThirdPersonGameMode.ThirdPersonGameMode_C|SetLevel _asthird_person_game_mode (+ (Variables|/Game/ThirdPersonBP/Blueprints/ThirdPersonGameMode.ThirdPersonGameMode_C|GetLevel _asthird_person_game_mode) 1))
    (Variables|/Game/ThirdPersonBP/Blueprints/ThirdPersonGameMode.ThirdPersonGameMode_C|SetExperience _asthird_person_game_mode 0)
    (Variables|/Game/ThirdPersonBP/Blueprints/ThirdPersonGameMode.ThirdPersonGameMode_C|SetMaxExperiance _asthird_person_game_mode (* (Variables|/Game/ThirdPersonBP/Blueprints/ThirdPersonGameMode.ThirdPersonGameMode_C|GetMaxExperiance _asthird_person_game_mode) 2))
    (bind _returnvalue (Game|ConstructObjectfromClass "/Game/ThirdPersonBP/Blueprints/LevelUp.LevelUp_C" (Game|GetPlayerCharacter 0)))
    (UserInterface|Viewport|AddtoViewport _returnvalue 0))
  (bind _asthird_person_game_mode_2 (Utilities|Casting|CastToThirdPersonGameMode (Game|GetGameMode)))
  (Default|UpdateNumbers _asthird_person_game_mode_2))